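; Player melee component for BP_ThirdPersonCharacter that runs a five-montage sword combo from the attack input.
; Presses during an attack are buffered in SaveAttack; SwordAttackCombo, called from outside, advances by AttackIndex or resets, with the fifth attack repeating while input continues.
; A looping timer sweeps sphere traces along the blade, and a separate trace covers kicks and lunges.
; Hits on "Damageable" actors apply damage, camera shake, sound and blood.
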(event `Attack 1`
  ;[0.05127 0.05127 0.05127] Combo System
  ;;[0.05127 0.05127 0.05127] Attack 1 - Don't forget to add anim notifies when adding different animations
  (`/Engine/EditorBlueprintResources/StandardMacros.DoOnce` false :!label _label
    (:`Completed`
      (`KismetSystemLibrary.Delay` 0.0)
      (`|PlayMontage` (`self.Character Mesh`) "/Game/Characters/RPG_Character/Animations/SwordAttacks/Combo_Attack_04_01_Seq_Montage.Combo_Attack_04_01_Seq_Montage"
        (:`then`
          (set `self.Attack Index` 1)
          (goto _label :!via `Reset`))))))

(event `Attack 2`
  ;[0.05127 0.05127 0.05127] Combo System
  ;;[0.05127 0.05127 0.05127] Attack 2 - https://youtu.be/sWpENaVGj2M?si=S1dCaGvJBFku2qOr
  (`/Engine/EditorBlueprintResources/StandardMacros.DoOnce` false :!label _label_2
    (:`Completed`
      (`KismetSystemLibrary.Delay` 0.1)
      (`|PlayMontage` (`self.Character Mesh`) "/Game/Characters/RPG_Character/Animations/SwordAttacks/Combo_Attack_03_02_Seq_Montage.Combo_Attack_03_02_Seq_Montage"
        (:`then`
          (set `self.Attack Index` 2)
          (goto _label_2 :!via `Reset`))))))

(event `self.ReceiveBeginPlay`
  ;[0.05127 0.05127 0.05127] Combo System
  (bind _asbp_third_person_character (cast `/Game/ThirdPerson/Blueprints/BP_ThirdPersonCharacter` (`self.GetOwner`)))
  (set `self.Character BP` _asbp_third_person_character)
  (set `self.Character Mesh` (`Character.Mesh` _asbp_third_person_character)))

(event `EnhancedInput|/Game/ThirdPerson/Input/Actions/IA_Attack`
  (params (ActionValue :type Boolean) (ElapsedSeconds :type "Float (double-precision)") (TriggeredSeconds :type "Float (double-precision)") (InputAction :type "InputAction Object Reference" :default "/Game/ThirdPerson/Input/Actions/IA_Attack.IA_Attack"))
  ;[0.05127 0.05127 0.05127] Combo System
  ;;[0.05127 0.05127 0.05127] Attack Input
  (:`Started`
    (if (`self.Can Attack?`)
      (`self.Sword Attack`))))

(event `Attack 3`
  ;[0.05127 0.05127 0.05127] Combo System
  ;;[0.05127 0.05127 0.05127] Attack 3
  (`/Engine/EditorBlueprintResources/StandardMacros.DoOnce` false :!label _label_3
    (:`Completed`
      (`KismetSystemLibrary.Delay` 0.1)
      (`|PlayMontage` (`self.Character Mesh`) "/Game/Characters/RPG_Character/Animations/SwordAttacks/Combo_Attack_03_03_Seq1_Montage.Combo_Attack_03_03_Seq1_Montage"
        (:`then`
          (set `self.Attack Index` 3)
          (goto _label_3 :!via `Reset`))))))

(event `Sword Attack`
  ;[0.05127 0.05127 0.05127] Combo System
  ;;[0.05127 0.05127 0.05127] Sword Attack
  (if (`self.IsAttacking?`)
    (set `self.SaveAttack?` true)
    (else
      (set `self.IsAttacking?` true)
      (switch `int` (`self.Attack Index`) :!label _label_4
        (:`0`
          (`self.Attack 1`))
        (:`1`
          (`self.Attack 2`))
        (:`2`
          (`self.Attack 3`))
        (:`3`
          (`self.Attack 4`))
        (:`4`
          (`self.Attack 5`))))))

(event `Attack 4`
  ;[0.05127 0.05127 0.05127] Combo System
  ;;[0.05127 0.05127 0.05127] Attack 4
  (`/Engine/EditorBlueprintResources/StandardMacros.DoOnce` false :!label _label_5
    (:`Completed`
      (`KismetSystemLibrary.Delay` 0.1)
      (`|PlayMontage` (`self.Character Mesh`) "/Game/Characters/RPG_Character/Animations/SwordAttacks/Combo_Attack_03_03_Seq_Montage.Combo_Attack_03_03_Seq_Montage"
        (:`then`
          (set `self.Attack Index` 4)
          (goto _label_5 :!via `Reset`))))))

(event `Sword Attack Combo`
  ;[0.05127 0.05127 0.05127] Combo System
  ;;[0.05127 0.05127 0.05127] Combo Continue
  (if (`self.SaveAttack?`)
    (set `self.SaveAttack?` false)
    (goto _label_4)
    (else
      (`self.Stop Combo`))))

(event `Attack 5`
  ;[0.05127 0.05127 0.05127] Combo System
  ;;[0.05127 0.05127 0.05127] Attack 5
  (`/Engine/EditorBlueprintResources/StandardMacros.DoOnce` false :!label _label_6
    (:`Completed`
      (`KismetSystemLibrary.Delay` 0.1)
      (`|PlayMontage` (`self.Character Mesh`) "/Game/Characters/RPG_Character/Animations/SwordAttacks/Combo_Attack_03_04_Seq_Montage.Combo_Attack_03_04_Seq_Montage"
        (:`then`
          (set `self.Attack Index` 4)
          (goto _label_6 :!via `Reset`))))))

(event `Stop Combo`
  ;[0.05127 0.05127 0.05127] Combo System
  ;;[0.05127 0.05127 0.05127] Stop Combo / Attack
  (set `self.IsAttacking?` false)
  (set `self.Attack Index` 0))

(event `Sphere Trace`
  (bind _returnvalue (`SceneComponent.K2_GetComponentLocation` (`/Game/ThirdPerson/Blueprints/BP_ThirdPersonCharacter.Sphere Trace` (`self.Character BP`))))
  ;[0.05127 0.05127 0.05127] Sphere Trace (For Kick & Lunge Strikes) https://youtu.be/zbbWk851IXk?si=GNBtxhIeh6_cQ8Yb&t=1468
  (bind (_outhit _returnvalue_2) (`KismetSystemLibrary.SphereTraceSingle` _returnvalue _returnvalue 25.0 "TraceTypeQuery1"))
  (if _returnvalue_2
    (bind (_bblockinghit _binitialoverlap _time _distance _location _impactpoint _normal _impactnormal _physmat _hitactor) (`GameplayStatics.BreakHitResult` _outhit))
    (if (`Actor.ActorHasTag` _hitactor "Damageable")
      (`GameplayStatics.ApplyDamage` _hitactor 10.0)
      (`GameplayStatics.PlayWorldCameraShake` "/Game/Blueprints/BP_SwordHitCameraShake.BP_SwordHitCameraShake_C" _location 0.0 2000.0)
      (`self.Play Sword Hit Sounds`)
      (`GameplayStatics.SpawnEmitterAtLocation` "/Game/VFXs/Particles/Blood/P_Blood_Splat_Cone.P_Blood_Splat_Cone" _location (`KismetMathLibrary.MakeRotFromXY` _normal _normal) (0.4 0.4 0.4) true "AutoRelease"))))

(event `Start Sword Trace`
  ;[0.05127 0.05127 0.05127] Sword Trace
  (bind _returnvalue (`KismetSystemLibrary.K2_SetTimerDelegate` (delegate `Sword Trace Loop`) 0.001 true))
  (set `self.SwordTraceLoop` _returnvalue))

(event `Sword Trace Loop`
  ;[0.05127 0.05127 0.05127] Sword Trace
  (bind (_outhit _returnvalue) (`KismetSystemLibrary.SphereTraceSingle` :`Start` (`SceneComponent.K2_GetComponentLocation` (`/Game/ThirdPerson/Blueprints/BP_ThirdPersonCharacter.Sword Top Point` (`self.Character BP`))) :`End` (`SceneComponent.K2_GetComponentLocation` (`/Game/ThirdPerson/Blueprints/BP_ThirdPersonCharacter.Sword Bottom Point` (`self.Character BP`))) :`Radius` 12.0 :`TraceChannel` "TraceTypeQuery1" :`DrawTime` 0.2))
  (if _returnvalue
    (bind (_bblockinghit _binitialoverlap _time _distance _location _impactpoint _normal _impactnormal _physmat _hitactor) (`GameplayStatics.BreakHitResult` _outhit))
    (if (`Actor.ActorHasTag` _hitactor "Damageable")
      (`/Engine/EditorBlueprintResources/StandardMacros.DoOnce` false :!label _label_7
        (:`Completed`
          (`GameplayStatics.ApplyDamage` _hitactor 10.0)
          (`GameplayStatics.PlayWorldCameraShake` "/Game/Blueprints/BP_SwordHitCameraShake.BP_SwordHitCameraShake_C" _location 0.0 2000.0)
          (`self.Play Sword Hit Sounds`)
          (`GameplayStatics.SpawnEmitterAtLocation` "/Game/VFXs/Particles/Blood/P_Blood_Splat_Cone.P_Blood_Splat_Cone" _location (`KismetMathLibrary.MakeRotFromXY` _normal _normal) (0.4 0.4 0.4) true "AutoRelease")
          (`KismetSystemLibrary.Delay` 0.5)
          (goto _label_7 :!via `Reset`))))))

(event `Stop Sword Trace`
  ;[0.05127 0.05127 0.05127] Sword Trace
  (`KismetSystemLibrary.K2_ClearAndInvalidateTimerHandle` (`self.SwordTraceLoop`)))

(event `Play Sword Hit Sounds`
  ;[0.05127 0.05127 0.05127] Play Sword Hit Sounds
  (`GameplayStatics.PlaySoundAtLocation` "/Game/Audio/Sword_Hits/MS_SwordHit.MS_SwordHit" (`Actor.K2_GetActorLocation` (`self.GetOwner`)) (struct) 1.0 1.0 0.0 "/Game/Audio/SA_Character.SA_Character" null null null))